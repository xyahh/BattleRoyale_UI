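; MyBaseCharacter is a character Blueprint that maps player input to weapon handling and an inventory UI.
; On BeginPlay it creates the Inventory_Widget, starts it closed and adds it to the viewport; holding the Inventory action shows it.
; Keys and mouse wheel drive the WeaponEquipment component to drop, store or cycle weapons.
; Number keys select weapons by index through the inventory widget rather than the component.
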(event EventBeginPlay
  (bind _returnvalue (UserInterface|CreateWidget "/Game/Widget/Inventory_Widget.Inventory_Widget_C" 0 self))
  (bind _output_get (Variables|Default|SetInventory _returnvalue))
  (Default|Open/Close _output_get false)
  (UserInterface|Viewport|AddtoViewport _output_get 0))

(event Input|ActionEvents|InputActionInventory
  (params (Key :type Key%20Structure :default "None"))
  (bind _inventory (Variables|Default|GetInventory))
  (:Pressed
    (Default|Open/Close _inventory true))
  (:Released
    (Default|Open/Close _inventory false)))

(event Input|KeyboardEvents|G
  (params (Key :type Key%20Structure :default "None"))
  (:Pressed
    (Class|WeaponEquipmentComponent|StoreCurrentWeapon (Variables|Default|GetWeaponEquipment))))

(event Input|MouseEvents|MouseWheelUp
  (params (Key :type Key%20Structure :default "None"))
  (:Pressed
    (Class|WeaponEquipmentComponent|SelectNextWeapon (Variables|Default|GetWeaponEquipment) 1)))

(event Input|KeyboardEvents|1
  (params (Key :type Key%20Structure :default "None"))
  (:Pressed
    (Default|SelectWeapon (Variables|Default|GetInventory))))

(event Input|KeyboardEvents|2
  (params (Key :type Key%20Structure :default "None"))
  (:Pressed
    (Default|SelectWeapon (Variables|Default|GetInventory) 1)))

(event Input|MouseEvents|MouseWheelDown
  (params (Key :type Key%20Structure :default "None"))
  (:Pressed
    (Class|WeaponEquipmentComponent|SelectNextWeapon (Variables|Default|GetWeaponEquipment) -1)))

(event Input|KeyboardEvents|Y
  (params (Key :type Key%20Structure :default "None"))
  (:Pressed
    (Class|WeaponEquipmentComponent|DropItem (Variables|Default|GetWeaponEquipment) (Class|WeaponEquipmentComponent|GetCurrentWeapon (Variables|Default|GetWeaponEquipment)))))

(fn ConstructionScript)